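; Player controller for the character select screen, handling menu input for joining and starting the game.
; Accept appends an entry to the Players array in PersintantVar_GameInstance on every press, logs the count and plays a click.
; Start plays a sound and opens MainLevel after a short delay, only if the controller's display name is exactly PC_SelectCharacter.
; Back only prints a debug message.
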(event EventBeginPlay)

(event EventTick
  (params (DeltaSeconds :type Float%20%28single-precision%29)))

(event Input|ActionEvents|InputActionBackMenu
  (params (Key :type Key%20Structure :default "None"))
  (:Pressed
    (Development|PrintString (Utilities|String|Append "he pulsado B" (Utilities|GetDisplayName self)))))

(event Input|ActionEvents|InputActionAcceptMenu
  (params (Key :type Key%20Structure :default "None"))
  (bind _returnvalue (Game|GetGameInstance))
  (bind _aspersintant_var_game_instance (Utilities|Casting|CastToPersintantVar_GameInstance _returnvalue))
  (bind _players (Variables|/Game/Blueprints/PersintantVar_GameInstance.PersintantVar_GameInstance_C|GetPlayers _aspersintant_var_game_instance))
  (:Pressed
    (Development|PrintString (Utilities|String|Append "he pulsado A" (Utilities|GetDisplayName self)))
    (Utilities|Array|Add _players true)
    (Development|PrintString (Utilities|String|ToString(Integer) (Utilities|Array|Length _players)))
    (Audio|SpawnSound2D "/Game/Music/Sonidos/click.click" 1.0 1.0 0.0 0)))

(event Input|ActionEvents|InputActionStartGame
  (params (Key :type Key%20Structure :default "None"))
  (:Pressed
    (if (Utilities|Enum|Equal(Enum) (Utilities|GetDisplayName self) "PC_SelectCharacter")
      (Audio|SpawnSound2D "/Game/Music/Sonidos/mover_menu.mover_menu" 1.0 1.0 0.0 0)
      (Utilities|FlowControl|Delay 0.5)
      (Game|OpenLevel(byName) "MainLevel"))))

(fn ConstructionScript)