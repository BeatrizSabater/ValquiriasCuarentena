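; Tall, narrow, single-sided store shelving unit that displays one randomly chosen product group, such as water, rice, milk or masks.
; Activate sets the Active flag and shows one of eighteen product group components by random roll over twenty values, so two outcomes show no products.
; Desactivate clears the flag and hides every group.
; The event graph and construction script hold no logic.
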(event EventBeginPlay)

(event Collision|EventActorBeginOverlap
  (params (OtherActor :type Actor%20Object%20Reference)))

(event EventTick
  (params (DeltaSeconds :type Float%20%28single-precision%29)))

(fn ConstructionScript)

(fn Activate
  (Variables|Default|SetActive true)
  (switch int (Math|Random|RandomInteger 20)
    (:0
      (Rendering|SetVisibility (Variables|Default|GetGrupoAgua) true false))
    (:1
      (Rendering|SetVisibility (Variables|Default|GetGrupoGuantes) true false))
    (:2
      (Rendering|SetVisibility (Variables|Default|GetGrupoMascarillas) true false))
    (:3
      (Rendering|SetVisibility (Variables|Default|GetGrupoPapelHigienico) true false))
    (:4
      (Rendering|SetVisibility (Variables|Default|GetGrupoArroz) true false))
    (:5
      (Rendering|SetVisibility (Variables|Default|GetGrupoBebidaAlcoholica) true false))
    (:6
      (Rendering|SetVisibility (Variables|Default|GetGrupoBebidaEnergetica) true false))
    (:7
      (Rendering|SetVisibility (Variables|Default|GetGrupoBotesAlargados) true false))
    (:8
      (Rendering|SetVisibility (Variables|Default|GetGrupoCajaCereales) true false))
    (:9
      (Rendering|SetVisibility (Variables|Default|GetGrupoCarne) true false))
    (:10
      (Rendering|SetVisibility (Variables|Default|GetGrupoDesinfectante) true false))
    (:11
      (Rendering|SetVisibility (Variables|Default|GetGrupoGarbanzos) true false))
    (:12
      (Rendering|SetVisibility (Variables|Default|GetGrupoHuevos) true false))
    (:13
      (Rendering|SetVisibility (Variables|Default|GetGrupoLatasRefrescos) true false))
    (:14
      (Rendering|SetVisibility (Variables|Default|GetGrupoLeche) true false))
    (:15
      (Rendering|SetVisibility (Variables|Default|GetGrupoMantequilla) true false))
    (:16
      (Rendering|SetVisibility (Variables|Default|GetGrupoNatillas) true false))
    (:17
      (Rendering|SetVisibility (Variables|Default|GetGrupoQueso) true false))))

(fn Desactivate
  (Variables|Default|SetActive false)
  (Rendering|SetVisibility (Variables|Default|GetGrupoAgua) false false)
  (Rendering|SetVisibility (Variables|Default|GetGrupoGuantes) false false)
  (Rendering|SetVisibility (Variables|Default|GetGrupoMascarillas) false false)
  (Rendering|SetVisibility (Variables|Default|GetGrupoPapelHigienico) false false)
  (Rendering|SetVisibility (Variables|Default|GetGrupoArroz) false false)
  (Rendering|SetVisibility (Variables|Default|GetGrupoBebidaAlcoholica) false false)
  (Rendering|SetVisibility (Variables|Default|GetGrupoBebidaEnergetica) false false)
  (Rendering|SetVisibility (Variables|Default|GetGrupoBotesAlargados) false false)
  (Rendering|SetVisibility (Variables|Default|GetGrupoCajaCereales) false false)
  (Rendering|SetVisibility (Variables|Default|GetGrupoCarne) false false)
  (Rendering|SetVisibility (Variables|Default|GetGrupoDesinfectante) false false)
  (Rendering|SetVisibility (Variables|Default|GetGrupoGarbanzos) false false)
  (Rendering|SetVisibility (Variables|Default|GetGrupoHuevos) false false)
  (Rendering|SetVisibility (Variables|Default|GetGrupoLatasRefrescos) false false)
  (Rendering|SetVisibility (Variables|Default|GetGrupoLeche) false false)
  (Rendering|SetVisibility (Variables|Default|GetGrupoMantequilla) false false)
  (Rendering|SetVisibility (Variables|Default|GetGrupoNatillas) false false)
  (Rendering|SetVisibility (Variables|Default|GetGrupoQueso) false false))